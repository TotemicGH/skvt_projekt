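; Base NPC character that takes damage with a hit montage and can be stealth-killed by the player.
; A box overlap shows the interaction to crouching players, while PawnSensing disables it on sight until a retriggerable delay lapses.
; The primary interaction triggers the player's stealth kill, plays a neck-break montage, then applies max-health damage.
; SkvtHealth death enables ragdoll physics, deactivates any assigned tutorial and destroys the actor after a timer.
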(event `self.ReceiveBeginPlay`)

(event `self.ReceiveTick`
  (params (DeltaSeconds :type "Float (single-precision)")))

(event `self.SkvtHealth.OnDeath`
  (bind _assignedtutorial (`self.AssignedTutorial`))
  (`PrimitiveComponent.SetSimulatePhysics` (`self.Mesh`) true)
  (`CharacterMovementComponent.DisableMovement` (`self.CharacterMovement`))
  (`KismetSystemLibrary.K2_SetTimerDelegate` (delegate `Destroy`) 5.0)
  (`/Engine/EditorBlueprintResources/StandardMacros.IsValid` _assignedtutorial
    (:`Is Valid`
      (`/Game/Skvt/Blueprints/Platform/BP_TutorialTrigger.Deactivate` _assignedtutorial))))

(event `Destroy`
  (`self.K2_DestroyActor`))

(event `self.ReceiveAnyDamage`
  (params (Damage :type "Float (single-precision)") (DamageType :type "DamageType Object Reference") (InstigatedBy :type "Controller Object Reference") (DamageCauser :type "Actor Object Reference"))
  (`/Game/Skvt/Systems/SkvtHealth.ProcessDamage` (`self.SkvtHealth`) Damage)
  (`self.PlayAnimMontage` "/Game/Skvt/Characters/Animations/Attacks/AM_Hit_punch.AM_Hit_punch"))

(event `self.PawnSensing.OnSeePawn`
  (params (Pawn :type "Pawn Object Reference"))
  (bind _skvtinteraction (`self.SkvtInteraction`))
  (`/Game/Skvt/Systems/SkvtInteraction.UpdateInteractionState` _skvtinteraction false false)
  (`KismetSystemLibrary.RetriggerableDelay` 0.6)
  (`/Game/Skvt/Systems/SkvtInteraction.UpdateInteractionState` _skvtinteraction true false))

(event `self.Box.OnComponentBeginOverlap`
  (params (OverlappedComponent :type "PrimitiveComponent Object Reference") (OtherActor :type "Actor Object Reference") (OtherComp :type "PrimitiveComponent Object Reference") (OtherBodyIndex :type Integer) (bFromSweep :type Boolean) (SweepResult :type "HitResult Structure (by ref)"))
  (bind _asbp_skvt_base_char (cast `/Game/Skvt/Characters/BP_SkvtBaseChar` OtherActor))
  (if (`NavMovementComponent.IsCrouching` (`Character.CharacterMovement` _asbp_skvt_base_char))
    (bind _asbp_skvt_player_controller (cast `/Game/Skvt/Characters/BP_SkvtPlayerController` (`self.GetController` _asbp_skvt_base_char)))
    (`/Game/Skvt/Systems/SkvtInteraction.ShowAvailableInteractions` (`self.SkvtInteraction`) _asbp_skvt_player_controller)))

(event `self.Box.OnComponentEndOverlap`
  (params (OverlappedComponent :type "PrimitiveComponent Object Reference") (OtherActor :type "Actor Object Reference") (OtherComp :type "PrimitiveComponent Object Reference") (OtherBodyIndex :type Integer))
  (bind _asbp_skvt_base_char (cast `/Game/Skvt/Characters/BP_SkvtBaseChar` OtherActor))
  (bind _asbp_skvt_player_controller (cast `/Game/Skvt/Characters/BP_SkvtPlayerController` (`self.GetController` _asbp_skvt_base_char)))
  (`/Game/Skvt/Systems/SkvtInteraction.HideAvailableInteractions` (`self.SkvtInteraction`) _asbp_skvt_player_controller))

(event `self.SkvtInteraction.OnInteractPrimary`
  (bind _asbp_skvt_base_char (cast `/Game/Skvt/Characters/BP_SkvtBaseChar` (`Controller.K2_GetPawn` (`/Game/Skvt/Systems/SkvtInteraction.PlayerController` (`self.SkvtInteraction`)))))
  (`/Game/Skvt/Systems/SkvtInteraction.UpdateInteractionState` (`self.SkvtInteraction`) false false)
  (`/Game/Skvt/Systems/PlayerInteractions.PerformStealthKill` (`/Game/Skvt/Characters/BP_SkvtBaseChar.PlayerInteractions` _asbp_skvt_base_char))
  (bind _returnvalue (`self.PlayAnimMontage` "/Game/Skvt/Characters/Animations/Attacks/AM_Hit_BreakNeck.AM_Hit_BreakNeck"))
  (`KismetSystemLibrary.Delay` _returnvalue)
  (`GameplayStatics.ApplyDamage` self (`/Game/Skvt/Systems/SkvtHealth.MaxHealth` (`self.SkvtHealth`))))

(fn `UserConstructionScript`)