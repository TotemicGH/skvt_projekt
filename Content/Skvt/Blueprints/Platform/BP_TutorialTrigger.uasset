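; Trigger volume that shows a tutorial widget of its WidgetType to players whose BP_SkvtBaseChar is inside its Box.
; Overlap begin, or a one-shot check shortly after BeginPlay for characters already inside, calls Activate immediately or after ActivationTime, provided IsActive is set.
; Activate and Deactivate toggle IsActive and show or hide the widget through BP_SkvtPlayerController for overlapping characters.
; Leaving the trigger also hides the widget.
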(event `self.ReceiveBeginPlay`
  (`KismetSystemLibrary.K2_SetTimerDelegate` (delegate `CheckOverlap`) 0.1))

(event `CheckOverlap`
  (bind _activationtime (`self.ActivationTime`))
  (if (> (`KismetArrayLibrary.Array_Length` (`PrimitiveComponent.GetOverlappingActors` (`self.Box`) "/Game/Skvt/Characters/BP_SkvtBaseChar.BP_SkvtBaseChar_C")) 0)
    (if (`self.IsActive`) :!label _label
      (if (> _activationtime 0.0)
        (`KismetSystemLibrary.K2_SetTimerDelegate` (delegate `ShowTutorial`) _activationtime)
        (else
          (`self.Activate` :!label _label_2))))))

(event `self.ReceiveActorBeginOverlap`
  (params (OtherActor :type "Actor Object Reference"))
  (goto _label))

(event `ShowTutorial`
  (if (`self.IsActive`)
    (goto _label_2)))

(event `self.ReceiveActorEndOverlap`
  (params (OtherActor :type "Actor Object Reference"))
  (bind _asbp_skvt_base_char (cast `/Game/Skvt/Characters/BP_SkvtBaseChar` OtherActor))
  (bind _asbp_skvt_player_controller (cast `/Game/Skvt/Characters/BP_SkvtPlayerController` (`Pawn.GetController` _asbp_skvt_base_char)))
  (`/Game/Skvt/Characters/BP_SkvtPlayerController.HideTutorialWidget` _asbp_skvt_player_controller))

(fn `Activate`
  (set `self.IsActive` true)
  (for _array_element (`PrimitiveComponent.GetOverlappingActors` (`self.Box`) "/Game/Skvt/Characters/BP_SkvtBaseChar.BP_SkvtBaseChar_C")
    (bind _asbp_skvt_base_char (cast `/Game/Skvt/Characters/BP_SkvtBaseChar` _array_element))
    (bind _asbp_skvt_player_controller (cast `/Game/Skvt/Characters/BP_SkvtPlayerController` (`Pawn.GetController` _asbp_skvt_base_char)))
    (`/Game/Skvt/Characters/BP_SkvtPlayerController.ShowTutorialWidget` _asbp_skvt_player_controller (`self.WidgetType`))))

(fn `Deactivate`
  (set `self.IsActive` false)
  (for _array_element (`PrimitiveComponent.GetOverlappingActors` (`self.Box`) "/Game/Skvt/Characters/BP_SkvtBaseChar.BP_SkvtBaseChar_C")
    (bind _asbp_skvt_base_char (cast `/Game/Skvt/Characters/BP_SkvtBaseChar` _array_element))
    (bind _asbp_skvt_player_controller (cast `/Game/Skvt/Characters/BP_SkvtPlayerController` (`Pawn.GetController` _asbp_skvt_base_char)))
    (`/Game/Skvt/Characters/BP_SkvtPlayerController.HideTutorialWidget` _asbp_skvt_player_controller)))

(fn `UserConstructionScript`)