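; Wall sconce light actor that can be toggled on and off and disabled by an EMP.
; The construction script applies visibility, brightness, color and cone angles to the light component.
; Toggle requests go through an internal function that only acts while the sconce has power.
; An EMP permanently cuts power and spawns a brief explosion effect, but clears power before its switch-off call, so that call leaves the light unchanged.
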(event `/Game/Skvt/Blueprints/BPI_Electric.ToggleOn`
  (params (IsOn :type Boolean))
  (`self.Toggle on Internal` IsOn))

(event `/Game/Skvt/Blueprints/BPI_Electric.TriggerEMP`
  (if (`self.HasElectricPower`)
    (set `self.HasElectricPower` false)
    (`self.Toggle on Internal` false)
    (bind _returnvalue (`GameplayStatics.SpawnEmitterAtLocation` "/Game/StarterContent/Particles/P_Explosion.P_Explosion" (`self.K2_GetActorLocation`) (struct) (0.3 0.3 0.3)))
    (`KismetSystemLibrary.Delay` 2.0)
    (`ActorComponent.K2_DestroyComponent` _returnvalue)))

(fn `Toggle on Internal`
  (params (IsOn :type Boolean))
  (if (`self.HasElectricPower`)
    (bind _output_get (set `self.IsOn` IsOn))
    (`SceneComponent.SetVisibility` (`self.SconceLight`) _output_get false)))

(fn `UserConstructionScript`
  (bind _sconcelight (`self.SconceLight`))
  (`SceneComponent.SetVisibility` _sconcelight (`self.IsOn`) false)
  (`LightComponent.SetIntensity` _sconcelight (`self.Brightness`))
  (`LightComponent.SetLightColor` _sconcelight (`self.Color`) true)
  (`SpotLightComponent.SetInnerConeAngle` _sconcelight (`self.Inner Cone Angle`))
  (`SpotLightComponent.SetOuterConeAngle` _sconcelight (`self.Outer Cone Angle`)))